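; LevelExit is an exit trigger actor that moves the player to the next level once they have a high enough score.
; On overlap, it checks that the other actor is the player and compares the Score on PlayerCharacter_BP to its ScoreNeeded variable.
; Meeting the threshold opens the hard-coded Level_2 map by name, while falling short prints a taunt message.
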(event `self.ReceiveActorBeginOverlap`
  (params (OtherActor :type "Actor Object Reference"))
  (if (== (`GameplayStatics.GetObjectClass` OtherActor) (`self.Player`))
    (bind _asplayer_character_bp (cast `/Game/Blueprints/Player_Character/PlayerCharacter_BP` OtherActor))
    (if (>= (`PlayerCharacter.Score` _asplayer_character_bp) (`self.ScoreNeeded`))
      (`GameplayStatics.OpenLevel` "Level_2")
      (else
        (`KismetSystemLibrary.PrintString` "You're not fat enough!")))))

(fn `UserConstructionScript`)