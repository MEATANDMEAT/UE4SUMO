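; AI controller Blueprint for an enemy that sets up patrol data and starts its behavior tree.
; On BeginPlay it prints a debug message, initializes the Patrol_AREA blackboard and writes random navigable locations to First Point and Second Point.
; Both points are searched around randomized origins near the world origin, independent of the pawn's position, before Behaviour_TREE runs.
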(event `self.ReceiveBeginPlay`
  (`KismetSystemLibrary.PrintString` "ENEMY NOW POSSESED BY AI CONTROLLER")
  (bind _blackboardcomponent (`self.UseBlackboard` "/Game/Patrol_AREA.Patrol_AREA"))
  (`BlackboardComponent.SetValueAsVector` _blackboardcomponent "First Point" (`NavigationSystem.K2_GetRandomLocationInNavigableRadius` (`KismetMathLibrary.MakeVector` (`KismetMathLibrary.RandomFloatInRange` 100.0 500.0) (`KismetMathLibrary.RandomFloatInRange` 100.0 500.0)) 20000.0))
  (`BlackboardComponent.SetValueAsVector` _blackboardcomponent "Second Point" (`NavigationSystem.K2_GetRandomLocationInNavigableRadius` (`KismetMathLibrary.MakeVector` (`KismetMathLibrary.RandomFloatInRange` 100.0 500.0) (`KismetMathLibrary.RandomFloatInRange` 100.0 500.0)) 20000.0))
  (`self.RunBehaviorTree` "/Game/Behaviour_TREE.Behaviour_TREE"))

(fn `UserConstructionScript`)