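; Shelf environment actor that gives its mesh a randomly tinted color based on its AllowSpawn flag.
; On BeginPlay, after a near-zero delay, it creates a dynamic material instance from ShelfMat and applies it to the static mesh.
; It then sets the Color parameter to a random reddish shade when AllowSpawn is true, or a blue-cyan shade otherwise.
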(event `self.ReceiveBeginPlay`
  (`KismetSystemLibrary.Delay` 0.0001)
  (bind _returnvalue (`KismetMaterialLibrary.CreateDynamicMaterialInstance` "/Game/ShelfMat.ShelfMat"))
  (`PrimitiveComponent.SetMaterial` (`self.WorldStaticMesh`) 0 _returnvalue)
  (if (`self.bAllowSpawn`)
    (`MeshComponent.SetVectorParameterValueOnMaterials` (`self.WorldStaticMesh`) "Color" (`KismetMathLibrary.MakeVector` (`KismetMathLibrary.RandomFloatInRange` 0.7 1.0) (`KismetMathLibrary.RandomFloatInRange` 0.0 0.2) (`KismetMathLibrary.RandomFloatInRange` 0.0 0.3)))
    (else
      (`MeshComponent.SetVectorParameterValueOnMaterials` (`self.WorldStaticMesh`) "Color" (`KismetMathLibrary.MakeVector` (`KismetMathLibrary.RandomFloatInRange` 0.0 0.3) (`KismetMathLibrary.RandomFloatInRange` 0.5 0.8) (`KismetMathLibrary.RandomFloatInRange` 0.7 1.0))))))

(fn `UserConstructionScript`)